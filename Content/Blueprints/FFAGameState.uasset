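; FFAGameState is a game state Blueprint, named for free-for-all play, that runs the round countdown.
; BeginPlay calls BeginRound, which sets RoundTime to five minutes in seconds and starts CountTimer.
; CountTimer decrements RoundTime and sets a one-second timer through a created event while time remains.
; No action follows when the count reaches zero.
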(event `self.ReceiveBeginPlay`
  (`self.BeginRound`))

(fn `BeginRound`
  (set `self.RoundTime` 300)
  (`self.CountTimer`))

(fn `CountTimer`
  (bind _roundtime (`self.RoundTime`))
  (if (> _roundtime 0)
    (set `self.RoundTime` (- _roundtime 1))
    (`KismetSystemLibrary.K2_SetTimerDelegate` (`|CreateDelegate` :!event `CountTimer`) 1.0)))

(fn `UserConstructionScript`)